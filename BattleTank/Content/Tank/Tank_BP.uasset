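; Player-controllable tank Blueprint that binds input to driving, aiming and firing.
; On BeginPlay it passes turret and barrel components to their reference setters and initialises TankMovement with both tracks.
; Driving works either through direct per-track throttle axes or through forward and turn intents sent to TankMovement.
; Aim axes rotate the azimuth gimbal in yaw and spring arm in pitch, while the Firing action calls Fire.
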(event `self.ReceiveBeginPlay`
  (`self.SetTurretReference` (`self.TankTurret`))
  (`self.SetBarrelReference` (`self.TankBarrel`))
  (`TankMovementComponent.Initialise` (`self.TankMovement`) (`self.Left Tank Track`) (`self.Right Tank Track`)))

(event `InputAxis|Left Track Throttle`
  (params (AxisValue :type "Float (single-precision)"))
  ;[1 1 1] Movement Input Binding
  (`TankTrack.SetThrottle` (`self.Left Tank Track`) AxisValue))

(event `InputAxis|AimAzimuth`
  (params (AxisValue :type "Float (single-precision)"))
  ;[1 1 1] Aiming Input Binding
  (`SceneComponent.K2_AddLocalRotation` (`self.AzimuthGimbal`) (`KismetMathLibrary.MakeRotator` 0.0 0.0 AxisValue) false false))

(event `InputAxis|Right Track Throttle`
  (params (AxisValue :type "Float (single-precision)"))
  ;[1 1 1] Movement Input Binding
  (`TankTrack.SetThrottle` (`self.Right Tank Track`) AxisValue))

(event `InputAxis|Forward`
  (params (AxisValue :type "Float (single-precision)"))
  ;[1 1 1] Movement Input Binding
  (`TankMovementComponent.IntendMoveForward` (`self.TankMovement`) AxisValue))

(event `InputAxis|AimAltitude`
  (params (AxisValue :type "Float (single-precision)"))
  ;[1 1 1] Aiming Input Binding
  (`SceneComponent.K2_AddLocalRotation` (`self.SpringArm`) (`KismetMathLibrary.MakeRotator` 0.0 AxisValue) false false))

(event `InputAxis|Turn Right`
  (params (AxisValue :type "Float (single-precision)"))
  ;[1 1 1] Movement Input Binding
  (`TankMovementComponent.IntendTurnRight` (`self.TankMovement`) AxisValue))

(event `InputAxis|Backward`
  (params (AxisValue :type "Float (single-precision)"))
  ;[1 1 1] Movement Input Binding
)

(event `InputAction|Firing`
  (params (Key :type "Key Structure"))
  ;[1 1 1] Aiming Input Binding
  (:`Pressed`
    (`self.Fire`)))

(fn `UserConstructionScript`)